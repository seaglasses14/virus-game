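; Protection component that tracks a breakable shield's hit points for its owner.
; BeginPlay calls Reset to fill current HP from max HP; Reset leaves the broken flag untouched.
; TakeDamage subtracts from HP, clamped at zero, only while a shield is present and unbroken.
; At zero it marks the shield broken and prints a message, without passing excess damage on.
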(event EventBeginPlay
  (CallFunction|Reset))

(event EventTick
  (params (DeltaSeconds :type Float%20%28single-precision%29)))

(fn TakeDamage
  (params (Amount :type Float%20%28double-precision%29))
  (if (and (Variables|Default|GetHas%20shield) (not (Variables|Default|GetIsbroken)))
    (bind _output_get (Variables|Default|SetCurrentHP (Math|Float|SelectFloat 0.0 (- (Variables|Default|GetCurrentHP) Amount) (<= (- (Variables|Default|GetCurrentHP) Amount) 0.0))))
    (if (<= _output_get 0.0)
      (Variables|Default|SetIsbroken true)
      (Development|PrintString "Shield Broken!"))))

(fn Reset
  (Variables|Default|SetCurrentHP (Variables|Default|GetMaxHP)))
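; Shield component for BP_VirusCharacter that tracks its own health and toggles the owner's shield mesh on and off.
; Damage counts only while the shield is active and unbroken, flashing the mesh's emissive color through a dynamic material instance and refreshing the owner's shield.
; At zero health it switches off and blocks toggling during a fixed cooldown, then restores health without reactivating itself.
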(event Custom|FlashShieldMesh
  (|SetFlashParametersON)
  (Utilities|FlowControl|Delay (Variables|Flashing|GetFlashDuration))
  (|SetFlashParametersOFF))

(event Custom|BreakShield
  (CallFunction|Enable/DisableShield)
  (Variables|Default|SetShieldBroken true)
  (Utilities|FlowControl|Delay 1e+01)
  (Variables|Default|SetShieldBroken false)
  (CallFunction|ResetHealth))

(event EventBeginPlay
  (bind _asbp_virus_character (Utilities|Casting|CastToBP_VirusCharacter (Components|GetOwner)))
  (Variables|Default|SetRefToOwner _asbp_virus_character)
  (CallFunction|ResetHealth)
  (Variables|Default|SetShieldMesh (Variables|/Game/Master/Player/Blueprints/BP_VirusCharacter.BP_VirusCharacter_C|GetShield (Variables|Default|GetRefToOwner)))
  (|SetMaterialToFlash))

(fn ResetHealth
  (Variables|Default|SetCurrentHealth (Variables|Default|GetMaxHealth)))

(fn TakeDamage
  (params (Amount :type Float%20%28double-precision%29))
  (if (and (Variables|Default|GetIsShieldActive) (not (Variables|Default|GetShieldBroken)))
    (bind _output_get (Variables|Default|SetCurrentHealth (Math|Float|SelectFloat 0.0 (- (Variables|Default|GetCurrentHealth) Amount) (<= (- (Variables|Default|GetCurrentHealth) Amount) 0.0))))
    (if (<= _output_get 0.0)
      (CallFunction|BreakShield)
      (else
        (CallFunction|FlashShieldMesh)
        (Default|RefreshShield (Variables|Default|GetRefToOwner))))))

(fn Enable/DisableShield
  (if (and (Variables|/Game/Master/Player/Blueprints/BP_VirusCharacter.BP_VirusCharacter_C|GetHasShield (Variables|Default|GetRefToOwner)) (not (Variables|Default|GetShieldBroken)))
    (Default|RefreshShield (Variables|Default|GetRefToOwner))
    (Rendering|SetVisibility (Variables|Default|GetShieldMesh) (not (Variables|Default|GetIsShieldActive)) true)
    (Variables|Default|SetIsShieldActive (not (Variables|Default|GetIsShieldActive)))))
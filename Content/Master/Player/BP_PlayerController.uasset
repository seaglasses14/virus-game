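; Player controller for a top-down game that moves BP_Player and turns its head toward the mouse cursor.
; BeginPlay caches the pawn as PlayerRef and adds the IMC_TopDown Enhanced Input context, whose IA_Move action drives movement relative to control rotation.
; Each Tick deprojects the mouse into a debug-drawn Visibility trace, stores CursorLocation and rotates the Head component toward it with pitch zeroed.
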(event EventBeginPlay
  (bind _returnvalue (PlayerController|LocalPlayerSubsystems|GetEnhancedInputLocalPlayerSubsystem))
  (CallFunction|GetPlayerRef)
  (Utilities|IsValid _returnvalue
    (:Is%20Valid
      (Input|AddMappingContext _returnvalue "/Game/Master/Input/IMC_TopDown.IMC_TopDown" 0 "(bIgnoreAllPressedKeysUntilRelease=True,bForceImmediately=False,bNotifyUserSettings=False)"))))

(event Input|EnhancedActionEvents|EnhancedInputActionIA_Move
  (params (ActionValue :type Vector%202D%20Structure) (ElapsedSeconds :type Float%20%28double-precision%29) (TriggeredSeconds :type Float%20%28double-precision%29) (InputAction :type Input%20Action%20Object%20Reference :default "/Game/Master/Input/Actions/IA_Move.IA_Move"))
  (bind _playerref (Variables|Default|GetPlayerRef))
  (bind _playerref_2 (Variables|Default|GetPlayerRef))
  (bind _returnvalue (Pawn|GetControlRotation _playerref :!class /Script/Engine.Pawn))
  (:Triggered
    (Pawn|Input|AddMovementInput _playerref (Math|Vector|GetRightVector (Math|Rotator|MakeRotator (.roll _returnvalue) 0.0 (.yaw _returnvalue))) (.x ActionValue) false)
    (Pawn|Input|AddMovementInput _playerref_2 (Math|Vector|GetForwardVector (Math|Rotator|MakeRotator 0.0 0.0 (.yaw (Pawn|GetControlRotation _playerref_2 :!class /Script/Engine.Pawn)))) (.y ActionValue) false)))

(event EventTick
  (params (DeltaSeconds :type Float%20%28single-precision%29))
  (bind (_locationx _locationy) (Game|Player|GetMousePosition))
  (bind _self self)
  (bind _playerref (Variables|Default|GetPlayerRef))
  (bind (_worldposition _worlddirection) (Class|GameplayStatics|DeprojectScreentoWorld _self (Math|Vector2D|MakeVector2D _locationx _locationy)))
  (bind _head (Variables|/Game/Master/Player/BP_Player.BP_Player_C|GetHead _playerref))
  (bind _outhit (Collision|LineTraceByChannel _worldposition (+ _worldposition (* _worlddirection 5e+03)) "TraceTypeQuery1" false 0 "ForDuration"))
  (if true
    (Variables|Default|SetCursorLocation (.Location (Collision|BreakHitResult _outhit)))
    (Transformation|SetWorldRotation _head (Math|Rotator|MakeRotator (.roll (Math|Rotator|FindLookatRotation (Transformation|GetWorldLocation _head) (.Location (Collision|BreakHitResult _outhit)))) 0.0 (.yaw (Math|Rotator|FindLookatRotation (Transformation|GetWorldLocation _head) (.Location (Collision|BreakHitResult _outhit))))) false false)))

(fn ConstructionScript)

(fn GetPlayerRef
  (bind _asbp_player (Utilities|Casting|CastToBP_Player (Game|Player|GetPlayerPawn 0)))
  (Variables|Default|SetPlayerRef _asbp_player))
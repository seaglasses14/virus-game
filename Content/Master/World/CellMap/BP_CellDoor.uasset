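; Cell map door that slides along Z when BP_VirusCharacter enters its trigger box and returns when the character leaves.
; A timeline, played and reversed on overlap, offsets the door from its initial location at a configurable rate.
; Unless AlreadyActive, it shows a text label and ignores the trigger channel until Activation hides the label and enables overlap.
; Construction places the label by IsRight; GetEnemyType and GetRandomPatrolPoint are stubs.
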(event OnComponentBeginOverlap(Box)
  (params (OverlappedComponent :type Primitive%20Component%20Object%20Reference) (OtherActor :type Actor%20Object%20Reference) (OtherComp :type Primitive%20Component%20Object%20Reference) (OtherBodyIndex :type Integer) (bFromSweep :type Boolean) (SweepResult :type Hit%20Result%20Structure%20%28by%20ref%29))
  (Utilities|Casting|CastToBP_VirusCharacter OtherActor)
  (CallFunction|DoorAnimationOpen))

(event OnComponentEndOverlap(Box)
  (params (OverlappedComponent :type Primitive%20Component%20Object%20Reference) (OtherActor :type Actor%20Object%20Reference) (OtherComp :type Primitive%20Component%20Object%20Reference) (OtherBodyIndex :type Integer))
  (Utilities|Casting|CastToBP_VirusCharacter OtherActor)
  (CallFunction|DoorAnimationClosed))

(event Custom|DoorAnimationClosed
  (bind _initdoorloc (Variables|Default|GetInitDoorLoc))
  (bind _doorposition (Timeline|DoorTimeline Reverse)
    (:Update
      (Transformation|SetRelativeLocation (Variables|Default|GetScene) (Math|Vector|MakeVector (.x _initdoorloc) (.y _initdoorloc) (+ (.z _initdoorloc) (* _doorposition (Variables|Default|GetZOffset)))) false false))))

(event Custom|DoorAnimationOpen
  (bind _initdoorloc (Variables|Default|GetInitDoorLoc))
  (bind _doorposition (Timeline|DoorTimeline Play)
    (:Update
      (Transformation|SetRelativeLocation (Variables|Default|GetScene) (Math|Vector|MakeVector (.x _initdoorloc) (.y _initdoorloc) (+ (.z _initdoorloc) (* _doorposition (Variables|Default|GetZOffset)))) false false))))

(event EventActivation
  (Collision|SetCollisionResponsetoChannel (Variables|Default|GetBox) "ECC_GameTraceChannel2" "ECR_Overlap")
  (Rendering|SetVisibility (Variables|Default|GetTextRender) false false))

(event EventBeginPlay
  (bind _alreadyactive (Variables|Default|GetAlreadyActive))
  (Components|Timeline|SetPlayRate (Variables|Default|GetDoorTimeline) (Variables|Default|GetDoorPlayRate))
  (Variables|Default|SetInitDoorLoc (Variables|/Script/Engine.SceneComponent|GetRelativeLocation (Variables|Default|GetScene)))
  (Rendering|SetVisibility (Variables|Default|GetTextRender) (not _alreadyactive) false)
  (Collision|SetCollisionResponsetoChannel (Variables|Default|GetBox) "ECC_GameTraceChannel2" (select _alreadyactive "ECR_Overlap" "ECR_Ignore")))

(fn ConstructionScript
  (bind _isright (Variables|Default|GetIsRight))
  (Transformation|SetRelativeLocationAndRotation (Variables|Default|GetTextRender) (Math|Vector|MakeVector 0.0 (Math|Float|SelectFloat -15.0 15.0 _isright) 0.0) (Math|Rotator|MakeRotator 0.0 0.0 (Math|Float|SelectFloat -9e+01 9e+01 _isright)) false false))

(fn GetEnemyType
  (return 0))

(fn GetRandomPatrolPoint
  (return "0, 0, 0"))
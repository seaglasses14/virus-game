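; Toxic hazard that damages the virus player character when it enters the hazard's box trigger.
; On begin overlap, it casts to BP_VirusCharacter and checks the character's ShieldComponent.
; An active, unbroken shield blocks the hit and only prints a debug message; otherwise the HealthComponent takes Damage.
; Damage applies once per entry, not over time, and passes a zero impact point.
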(event OnComponentBeginOverlap(Box)
  (params (OverlappedComponent :type Primitive%20Component%20Object%20Reference) (OtherActor :type Actor%20Object%20Reference) (OtherComp :type Primitive%20Component%20Object%20Reference) (OtherBodyIndex :type Integer) (bFromSweep :type Boolean) (SweepResult :type Hit%20Result%20Structure%20%28by%20ref%29))
  (bind _asbp_virus_character (Utilities|Casting|CastToBP_VirusCharacter OtherActor))
  (if (and (Variables|/Game/Master/Utilities/Components/BP_ShieldComponent.BP_ShieldComponent_C|GetIsShieldActive (Variables|/Game/Master/Player/Blueprints/BP_VirusCharacter.BP_VirusCharacter_C|GetShieldComponent _asbp_virus_character)) (not (Variables|/Game/Master/Utilities/Components/BP_ShieldComponent.BP_ShieldComponent_C|GetShieldBroken (Variables|/Game/Master/Player/Blueprints/BP_VirusCharacter.BP_VirusCharacter_C|GetShieldComponent _asbp_virus_character))))
    (Development|PrintString "Protected")
    (else
      (Default|TakeDamage (Variables|/Game/Master/Player/Blueprints/BP_VirusCharacter.BP_VirusCharacter_C|GetHealthComponent _asbp_virus_character) (Variables|Default|GetDamage) "0, 0, 0"))))

(fn ConstructionScript)
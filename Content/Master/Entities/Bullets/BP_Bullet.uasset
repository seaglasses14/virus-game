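; Pooled bullet actor that starts dormant, is activated with a data asset, transform and direction, and moves by a swept offset each tick.
; Activation swaps two trace-channel responses for player or non-player shots and applies the data asset's material.
; On hit, it sends a damage message to actors with a health component, then hides, disables collision and tick, and signals that it is free for reuse.
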(event OnComponentHit(Body)
  (params (HitComponent :type Primitive%20Component%20Object%20Reference) (OtherActor :type Actor%20Object%20Reference) (OtherComp :type Primitive%20Component%20Object%20Reference) (NormalImpulse :type Vector :default "0, 0, 0") (Hit :type Hit%20Result%20Structure%20%28by%20ref%29))
  (Utilities|IsValid (Actor|GetComponentbyClass OtherActor "/Game/Master/Utilities/Components/BP_HealthComponent.BP_HealthComponent_C")
    (:Is%20Valid
      (Class|BPIWorldActors|SelectDamage(Message) OtherActor (Variables|Default|GetDamage) (Transformation|GetWorldLocation (Variables|Default|GetBody)) false))
    (:Is%20Not%20Valid
      _))
  (CallFunction|DeactivateEntity)
  (Default|CallFreeBulletSignal self))

(event EventTick
  (params (DeltaSeconds :type Float%20%28single-precision%29))
  (Transformation|AddActorWorldOffset (* (Variables|Default|GetDirection) (Variables|/Game/Master/Entities/Bullets/BP_DA_B_BulletData.BP_DA_B_BulletData_C|GetSpeed (Variables|Default|GetBulletDataAsset)) DeltaSeconds) true))

(event EventBeginPlay
  (CallFunction|DeactivateEntity))

(fn ConstructionScript)

(fn ActivateEntity
  (params (NewDataAsset :type BP%20DA%20B%20Bullet%20Data%20Object%20Reference) (Location :type Vector) (Rotation :type Rotator) (Direction :type Vector) (IsPlayer :type Boolean))
  (bind _body (Variables|Default|GetBody))
  (bind _body_2 (Variables|Default|GetBody))
  (if IsPlayer
    (Collision|SetCollisionResponsetoChannel _body_2 "ECC_GameTraceChannel1" "ECR_Block")
    (Collision|SetCollisionResponsetoChannel _body_2 "ECC_GameTraceChannel2" "ECR_Ignore")
    (else
      (Collision|SetCollisionResponsetoChannel _body "ECC_GameTraceChannel1" "ECR_Ignore")
      (Collision|SetCollisionResponsetoChannel _body "ECC_GameTraceChannel2" "ECR_Block")))
  (Transformation|SetWorldLocationAndRotation (Variables|Default|GetBody) Location Rotation false false)
  (Variables|Default|SetBulletDataAsset NewDataAsset)
  (Variables|Default|SetDirection Direction)
  (Utilities|FlowControl|Sequence
    (:then_0
      (Rendering|Material|SetMaterial (Variables|Default|GetBody) 0 (Variables|/Game/Master/Entities/Bullets/BP_DA_B_BulletData.BP_DA_B_BulletData_C|GetMaterial (Variables|Default|GetBulletDataAsset))))
    (:then_1
      (Rendering|SetActorHiddenInGame false)
      (Collision|SetCollisionEnabled (Variables|Default|GetBody) "QueryAndPhysics")
      (Actor|Tick|SetActorTickEnabled true))))

(fn DeactivateEntity
  (Rendering|SetActorHiddenInGame true)
  (Collision|SetCollisionEnabled (Variables|Default|GetBody) "NoCollision")
  (Actor|Tick|SetActorTickEnabled false))
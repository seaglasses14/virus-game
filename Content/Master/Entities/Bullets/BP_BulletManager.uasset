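; BP_BulletManager is an object pool for bullets, spawning them when the player's BP_VirusCharacter signals a shot.
; On BeginPlay it pre-spawns MaxSize BP_Bullet actors into a free list and binds each one's free signal to return it there.
; Spawn requests activate a free bullet with a data asset, transform, direction and owner flag.
; When none are free, it recycles the oldest active bullet.
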(event Custom|InitializePool
  (for _index (range 0 (- (Variables|Default|GetMaxSize) 1))
    (bind _returnvalue (Game|SpawnActorfromClass "/Game/Master/Entities/Bullets/BP_Bullet.BP_Bullet_C" (Transformation|GetWorldTransform (Variables|Default|GetDefaultSceneRoot)) "AlwaysSpawn" "MultiplyWithRoot" 0 0))
    (EventDispatchers|BindEventtoFreeBulletSignal _returnvalue (delegate Custom|FreeBullet))
    (Utilities|Array|Add (Variables|Default|GetFreeBullets) _returnvalue)))

(event Custom|FreeBullet
  (params (Bullet :type BP%20Bullet%20Object%20Reference))
  (Utilities|Array|RemoveItem (Variables|Default|GetActiveBullets) Bullet)
  (Utilities|Array|Add (Variables|Default|GetFreeBullets) Bullet))

(event Custom|SpawnBullet
  (params (BulletDataAsset :type BP%20DA%20B%20Bullet%20Data%20Object%20Reference) (Location :type Vector) (Rotation :type Rotator) (Direction :type Vector) (IsPlayer :type Boolean))
  (bind _activebullets (Variables|Default|GetActiveBullets))
  (bind _freebullets (Variables|Default|GetFreeBullets))
  (bind _output_get (Variables|Default|SetTempSpawn (Utilities|Array|Get(acopy) _freebullets)))
  (Utilities|IsValid _output_get
    (:Is%20Valid
      (Default|ActivateEntity _output_get BulletDataAsset Location Rotation Direction IsPlayer)
      (Utilities|Array|RemoveIndex _freebullets)
      (Utilities|Array|Add (Variables|Default|GetActiveBullets) _output_get))
    (:Is%20Not%20Valid
      (bind _output_get_2 (Variables|Default|SetTempRemove (Utilities|Array|Get(acopy) (Variables|Default|GetActiveBullets))))
      (Utilities|IsValid _output_get_2
        (:Is%20Valid
          (Default|DeactivateEntity _output_get_2)
          (Utilities|Array|RemoveItem _activebullets _output_get_2)
          (Utilities|Array|Add _activebullets _output_get_2)
          (Default|ActivateEntity _output_get_2 BulletDataAsset Location Rotation Direction IsPlayer))
        (:Is%20Not%20Valid
          (Development|PrintString "BP_BulletManager/Event Graph:\\nImpossible"))))))

(event EventBeginPlay
  (bind _asbp_virus_character (Utilities|Casting|CastToBP_VirusCharacter (Game|Player|GetPlayerPawn 0)))
  (EventDispatchers|BindEventtoSpawnBullet _asbp_virus_character (delegate Custom|SpawnBullet))
  (CallFunction|InitializePool))

(fn ConstructionScript)
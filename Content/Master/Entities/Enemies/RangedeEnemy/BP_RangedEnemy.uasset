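; Ranged enemy Blueprint that extends a parent enemy's attack events to fire bullets at the player character.
; SetIsAttacking turns the actor toward the player on the horizontal plane and starts a looping Shoot timer if none is active.
; Shoot spawns bullets through BulletManager from AimPoint along its forward vector, using the DA_RangedEnemy data asset.
; Any SetBTAttackStatus call clears the timer after running parent logic, regardless of PlayerIsHere.
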(event Custom|Shoot
  (bind _aimpoint (Variables|Default|GetAimPoint))
  (Default|SpawnBullet (Variables|Default|GetBulletManager) "/Game/Master/Entities/Enemies/RangedeEnemy/DA_RangedEnemy.DA_RangedEnemy" (Transformation|GetWorldLocation _aimpoint) (Transformation|GetWorldRotation _aimpoint) (Math|Vector|GetForwardVector _aimpoint) false))

(event EventSetIsAttacking
  (bind _mesh (Variables|Character|GetMesh))
  (bind _reftocharacter (Variables|Default|GetRefToCharacter))
  (bind _returnvalue (Transformation|GetActorLocation _reftocharacter))
  (bind _returnvalue_2 (Transformation|GetWorldLocation _mesh))
  (|CallParentFunction)
  (Transformation|SetActorRotation (Math|Rotator|FindLookatRotation (Math|Vector|MakeVector (.x _returnvalue_2) (.y _returnvalue_2) (.z _returnvalue_2)) (Math|Vector|MakeVector (.x _returnvalue) (.y _returnvalue) (.z _returnvalue_2))))
  (if (not (Utilities|Time|IsTimerActivebyHandle (Variables|Default|GetTimerHandle)))
    (bind _returnvalue_3 (Utilities|Time|SetTimerbyEvent (delegate Custom|Shoot) 0.5 true))
    (Variables|Default|SetTimerHandle _returnvalue_3)))

(event EventSetBTAttackStatus
  (params (PlayerIsHere :type Boolean))
  (|CallParentFunction PlayerIsHere)
  (Utilities|Time|ClearandInvalidateTimerbyHandle (Variables|Default|GetTimerHandle)))

(fn ConstructionScript)
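; Base enemy character with patrol, chase and attack support for a behavior tree, via a blackboard attack flag that also switches walk and chase speed.
; Incoming damage hits an unbroken shield component first, at half strength unless from a laser, otherwise the health component.
; Health changes launch the enemy horizontally away from the impact point.
; Its PatrolArea supplies random navigable patrol points and is notified on death before the actor is destroyed.
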(event Custom|Knockback
  (params (MaxHealth :type Float%20%28double-precision%29) (CurrentHealth :type Float%20%28double-precision%29) (IsDead :type Boolean) (ImpactPoint :type Vector))
  (Character|LaunchCharacter (* (* 7.5e+02 (Math|Vector|Normalize (- (Transformation|GetActorLocation) ImpactPoint))) "1.000000,1.000000,0.000000") false false))

(event EventSetBTAttackStatus
  (params (PlayerIsHere :type Boolean))
  ;[1 1 1] Sets BT Status to attack and executes the task
  (AI|Components|Blackboard|SetValueasBool (AI|GetBlackboard 0) (Variables|Attack|GetAttackKeyName) PlayerIsHere)
  (Variables|/Script/Engine.CharacterMovementComponent|SetMaxWalkSpeed (Variables|Character|GetCharacterMovement) (Math|Float|SelectFloat (Variables|Movement|GetChaseSpeed) (Variables|Movement|GetWalkSpeed) PlayerIsHere)))

(event EventSelectDamage
  (params (Amount :type Float%20%28double-precision%29) (InpactPoint :type Vector :default "0, 0, 0") (IsLaser :type Boolean))
  (bind _bp_protectioncomponent (Variables|Default|GetBP_ProtectionComponent))
  ;[1 1 1] Check if has protection or not and take damage
  (if (and (Variables|/Game/Master/Utilities/Components/BP_ProtectionComponent.BP_ProtectionComponent_C|GetHas%20shield _bp_protectioncomponent) (not (Variables|/Game/Master/Utilities/Components/BP_ProtectionComponent.BP_ProtectionComponent_C|GetIsbroken _bp_protectioncomponent)))
    (Default|TakeDamage (Variables|Default|GetBP_ProtectionComponent) (|CheckIfCanDamageProtection Amount IsLaser))
    (else
      (Default|TakeDamage (Variables|Default|GetBP_HealthComponent) Amount InpactPoint))))

(event EventBeginPlay
  (bind _asbp_virus_character (Utilities|Casting|CastToBP_VirusCharacter (Game|GetPlayerCharacter 0)))
  (Variables|Base|SetRefToCharacter _asbp_virus_character)
  (EventDispatchers|BindEventtoOnHealthChanged (Variables|Default|GetBP_HealthComponent) (delegate Custom|Knockback)))

(event EventSetIsAttacking
  ;[1 1 1] Triggers attack animation
  (Variables|Attack|SetIsAttacking true))

(fn ConstructionScript)

(fn OnDeath
  (Default|EnemyDead (Variables|Base|GetPatrolArea))
  (Actor|DestroyActor))

(fn GetEnemyType
  (return (Variables|Base|GetType)))

(fn GetRandomPatrolPoint
  (bind _patrolarea (Variables|Base|GetPatrolArea))
  (bind _sphere (Variables|/Game/Master/Entities/Enemies/BP_EnemySpawner.BP_EnemySpawner_C|GetSphere _patrolarea))
  (Utilities|IsValid _patrolarea
    (:Is%20Valid
      (bind _randomlocation (Class|NavigationSystemV1|GetRandomLocationinNavigableRadius (Transformation|GetWorldLocation _sphere) (Variables|/Script/Engine.SphereComponent|GetSphereRadius _sphere) 0 0))
      (return _randomlocation))
    (:Is%20Not%20Valid
      (Development|PrintString "No PatrolArea Selected"))))
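; BP_RangedEnemy is an enemy that turns toward the player and fires bullets on a repeating timer while attacking.
; Attacking rotates it on yaw only, by matching the target height to its mesh, then starts a looping Shoot timer if none is active.
; Shoot spawns bullets from AimPoint through BulletManager using DA_RangedEnemy data.
; Setting the behavior tree attack status calls the parent and clears the timer, stopping fire.
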(event Custom|Shoot
  (bind _aimpoint (Variables|Default|GetAimPoint))
  (Default|SpawnBullet (Variables|Default|GetBulletManager) "/Game/Master/Entities/Enemies/RangedEnemy/DA_RangedEnemy.DA_RangedEnemy" (Transformation|GetWorldLocation _aimpoint) (Transformation|GetWorldRotation _aimpoint) (Math|Vector|GetForwardVector _aimpoint) false))

(event EventSetIsAttacking
  (|CallParentFunction)
  (|FaceThePlayer)
  (if (not (Utilities|Time|IsTimerActivebyHandle (Variables|Default|GetTimerHandle)))
    (bind _returnvalue (Utilities|Time|SetTimerbyEvent (delegate Custom|Shoot) 1.5 true))
    (Variables|Default|SetTimerHandle _returnvalue)))

(event EventSetBTAttackStatus
  (params (PlayerIsHere :type Boolean))
  ;[1 1 1] Triggers the BT Attack Status
  (|CallParentFunction PlayerIsHere)
  (Utilities|Time|ClearandInvalidateTimerbyHandle (Variables|Default|GetTimerHandle)))

(fn ConstructionScript)
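; Enemy spawner area that tells enemies when the player enters or leaves its fall-off sphere; no spawning logic appears in these graphs.
; The construction script sizes an inner sphere to SpawnRadius and the outer one larger by FallOffPercent, clamped between zero and one.
; Player entry sends attack status to valid members of the Enemies array, while exit sends it only to enemies still overlapping the outer sphere.
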(event OnComponentBeginOverlap(SphereFallOff)
  (params (OverlappedComponent :type Primitive%20Component%20Object%20Reference) (OtherActor :type Actor%20Object%20Reference) (OtherComp :type Primitive%20Component%20Object%20Reference) (OtherBodyIndex :type Integer) (bFromSweep :type Boolean) (SweepResult :type Hit%20Result%20Structure%20%28by%20ref%29))
  (if (== OtherActor (Game|GetPlayerCharacter 0))
    (bind _output_get (Variables|Default|SetPlayerIsHere true))
    (for _array_element (Variables|Default|GetEnemies)
      (Utilities|IsValid _array_element
        (:Is%20Valid
          (Class|BPIWorldActors|SetBTAttackStatus(Message) _array_element _output_get))))))

(event OnComponentEndOverlap(SphereFallOff)
  (params (OverlappedComponent :type Primitive%20Component%20Object%20Reference) (OtherActor :type Actor%20Object%20Reference) (OtherComp :type Primitive%20Component%20Object%20Reference) (OtherBodyIndex :type Integer))
  (if (== OtherActor (Game|GetPlayerCharacter 0))
    (bind _output_get (Variables|Default|SetPlayerIsHere false))
    (for _array_element (Collision|GetOverlappingActors (Variables|Default|GetSphereFallOff) "/Game/Master/Entities/Enemies/BP_EnemyParent.BP_EnemyParent_C" :!class /Script/Engine.PrimitiveComponent)
      (Class|BPIWorldActors|SetBTAttackStatus(Message) _array_element _output_get))))

(fn ConstructionScript
  (bind _spawnradius (Variables|Default|GetSpawnRadius))
  (CallFunction|MapFallOffPercent)
  (Components|Sphere|SetSphereRadius (Variables|Default|GetSphere) (Variables|Default|GetSpawnRadius) true)
  (Components|Sphere|SetSphereRadius (Variables|Default|GetSphereFallOff) (+ _spawnradius (* _spawnradius (Variables|Default|GetFallOffPercent))) true))

(fn MapFallOffPercent
  (if (> (Variables|Default|GetFallOffPercent) 1.0)
    (Variables|Default|SetFallOffPercent 1.0)
    (elif (< (Variables|Default|GetFallOffPercent) 0.0)
      (Variables|Default|SetFallOffPercent 0.0))))
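; Base enemy character that patrols an assigned PatrolArea and changes behavior when the player is inside it.
; Each tick it copies the area's PlayerIsHere flag to the IsPlayerNearby blackboard key and switches between chase and walk speed.
; GetRandomPatrolPoint returns random navigable locations within the area's sphere, and SetIsAttacking disables movement while flagging the attack animation.
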(event EventTick
  (params (DeltaSeconds :type Float%20%28single-precision%29))
  (bind _patrolarea (Variables|Default|GetPatrolArea))
  (bind _playerishere (Variables|/Game/Master/Entities/Enemies/BP_EnemySpawner.BP_EnemySpawner_C|GetPlayerIsHere _patrolarea))
  ;[1 1 1] Check if can Attack the player and enable BT status
  (AI|Components|Blackboard|SetValueasBool (AI|GetBlackboard 0) (Utilities|Name|MakeLiteralName "IsPlayerNearby") _playerishere)
  (Variables|/Script/Engine.CharacterMovementComponent|SetMaxWalkSpeed (Variables|Character|GetCharacterMovement) (Math|Float|SelectFloat (Variables|Default|GetChaseSpeed) (Variables|Default|GetWalkSpeed) _playerishere)))

(event EventSetIsAttacking
  ;[1 1 1] Triggers attack animation
  (Variables|Default|SetIsAttacking true)
  (Pawn|Components|CharacterMovement|DisableMovement (Variables|Character|GetCharacterMovement)))

(event EventBeginPlay
  (bind _asbp_virus_character (Utilities|Casting|CastToBP_VirusCharacter (Game|GetPlayerCharacter 0)))
  (Variables|Default|SetRefToCharacter _asbp_virus_character))

(fn ConstructionScript)

(fn GetEnemyType
  (return (Variables|Default|GetType)))

(fn GetRandomPatrolPoint
  (bind _patrolarea (Variables|Default|GetPatrolArea))
  (bind _sphere (Variables|/Game/Master/Entities/Enemies/BP_EnemySpawner.BP_EnemySpawner_C|GetSphere _patrolarea))
  (Utilities|IsValid _patrolarea
    (:Is%20Valid
      (bind _randomlocation (Class|NavigationSystemV1|GetRandomLocationinNavigableRadius (Transformation|GetWorldLocation _sphere) (Variables|/Script/Engine.SphereComponent|GetSphereRadius _sphere) 0 0))
      (return _randomlocation))
    (:Is%20Not%20Valid
      (Development|PrintString "No PatrolArea Selected"))))
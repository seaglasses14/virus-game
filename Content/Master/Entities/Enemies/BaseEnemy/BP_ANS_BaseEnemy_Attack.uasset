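; Anim notify state for BP_BaseEnemy attack animations that applies melee damage and closes out the attack.
; On begin, it makes a single overlap check of the enemy's MeleeSphere for RefToCharacter and, if found, calls SelectDamage with the enemy's Damage and the sphere's location.
; On end, it clears IsAttacking and sets the enemy's movement mode back to Walking.
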(fn ReceivedNotifyBegin
  (params (MeshComp :type Skeletal%20Mesh%20Component%20Object%20Reference) (Animation :type Anim%20Sequence%20Base%20Object%20Reference) (TotalDuration :type Float%20%28single-precision%29) (EventReference :type Anim%20Notify%20Event%20Reference%20Structure%20%28by%20ref%29))
  (bind _asbp_base_enemy (Utilities|Casting|CastToBP_BaseEnemy (Components|GetOwner MeshComp)))
  (if (Utilities|Array|ContainsItem (Collision|GetOverlappingActors (Variables|/Game/Master/Entities/Enemies/BaseEnemy/BP_BaseEnemy.BP_BaseEnemy_C|GetMeleeSphere _asbp_base_enemy) 0 :!class /Script/Engine.PrimitiveComponent) (Variables|/Game/Master/Entities/Enemies/BP_EnemyParent.BP_EnemyParent_C|GetRefToCharacter _asbp_base_enemy))
    (Default|SelectDamage (Variables|/Game/Master/Entities/Enemies/BP_EnemyParent.BP_EnemyParent_C|GetRefToCharacter _asbp_base_enemy) (Variables|/Game/Master/Entities/Enemies/BP_EnemyParent.BP_EnemyParent_C|GetDamage _asbp_base_enemy) (Transformation|GetWorldLocation (Variables|/Game/Master/Entities/Enemies/BaseEnemy/BP_BaseEnemy.BP_BaseEnemy_C|GetMeleeSphere _asbp_base_enemy))))
  (return false))

(fn ReceivedNotifyEnd
  (params (MeshComp :type Skeletal%20Mesh%20Component%20Object%20Reference) (Animation :type Anim%20Sequence%20Base%20Object%20Reference) (EventReference :type Anim%20Notify%20Event%20Reference%20Structure%20%28by%20ref%29))
  (bind _asbp_base_enemy (Utilities|Casting|CastToBP_BaseEnemy (Components|GetOwner MeshComp)))
  (Variables|/Game/Master/Entities/Enemies/BP_EnemyParent.BP_EnemyParent_C|SetIsAttacking _asbp_base_enemy false)
  (Pawn|Components|CharacterMovement|SetMovementMode (Variables|/Script/Engine.Character|GetCharacterMovement _asbp_base_enemy) "MOVE_Walking" 0)
  (return false))